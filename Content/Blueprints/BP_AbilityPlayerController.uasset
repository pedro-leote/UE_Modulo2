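; Player controller that casts the main attack at the location under the cursor.
; The IA_AbilityOne_Keyboard input event caches the cursor hit location and spawns BP_MainAttack just above it, with the player character as instigator and a short lifespan.
; BeginPlay and Tick only call the parent, and a note suggests the spawn logic may move to a player character function.
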(event `self.ReceiveBeginPlay`
  (`parent.ReceiveBeginPlay`))

(event `self.ReceiveTick`
  (params (DeltaSeconds :type "Float (single-precision)"))
  (`parent.ReceiveTick` 0.0))

(event `EnhancedInput|/Game/Input/IA_AbilityOne_Keyboard`
  (params (ActionValue :type Boolean) (ElapsedSeconds :type "Float (double-precision)") (TriggeredSeconds :type "Float (double-precision)") (InputAction :type "InputAction Object Reference" :default "/Game/Input/IA_AbilityOne_Keyboard.IA_AbilityOne_Keyboard"))
  (bind (_hit _location) (`self.GetLocationUnderCursor`))
  ; Change with Player Character called function maybe
  (:`Triggered`
    (if _hit
      (bind _output_get (set `self.Cached Destination` _location))
      (bind _returnvalue (`|SpawnActorFromClass` "/Game/Blueprints/BP_MainAttack.BP_MainAttack_C" (`KismetMathLibrary.Conv_VectorToTransform` (`KismetMathLibrary.MakeVector` (.x _output_get) (.y _output_get) (+ (.z _output_get) 0.05))) "Undefined" "MultiplyWithRoot" null (`GameplayStatics.GetPlayerCharacter` 0)))
      (`self.SetLifeSpan` _returnvalue 4.0))))

(fn `UserConstructionScript`)